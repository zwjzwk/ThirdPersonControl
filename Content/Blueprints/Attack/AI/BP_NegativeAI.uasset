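; Samurai enemy AI character that runs BT_NegativeAI against the player character, with sword equip, random combo or dodge attacks, and sphere-trace damage.
; Looping random-interval timers trigger blocking, strafing and two gap-closing special attacks that lerp toward the target via timelines.
; Damage plays block, random dodge or heavy-hit reactions, reduces HP, and on death ragdolls then destroys the actor.
; Tick keeps it facing the target and applies strafe input.
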(event Custom|Attack
  ;[1 1 1] 攻击
  (if (not (or (Variables|Default|GetAttackMontage) (Variables|Default|GetHitMontagePlay)))
    (Variables|Default|SetAttackMontage true)
    (if (== (Math|Random|RandomIntegerinRange 0 6) 0)
      (Variables|Default|SetDodgeMontagePlay true)
      (Animation|Montage|PlayMontage (Variables|Character|GetMesh) "/Game/GhostSamurai_Katana/GhostSamurai_Katana/Animation/Apose/Dodge/Root/GhostSamurai_APose_Dodge_B_Root_Montage.GhostSamurai_APose_Dodge_B_Root_Montage"
        (:OnBlendOut
          (Variables|Default|SetDodgeMontagePlay false)))
      (else
        (Animation|Montage|PlayMontage (Variables|Character|GetMesh) (Utilities|Array|Get(acopy) (Variables|Default|GetAttack%20Montage%20to%20Play) (Math|Random|RandomIntegerinRange 0 4)))))))

(event Custom|ResetAttack
  ;[1 1 1] 重置攻击
  (Variables|Default|SetAttackMontage false)
  (Variables|Default|SetDodgeMontagePlay false))

(event Custom|SpecialAttackSphere
  (bind _arrow1 (Variables|Default|GetArrow1))
  (bind _returnvalue (Transformation|GetWorldLocation _arrow1))
  ;[1 1 1] 特殊攻击范围检测
  (bind (_outhits _returnvalue_2) (Collision|MultiSphereTraceByChannel _returnvalue (+ _returnvalue (* (Math|Vector|GetForwardVector _arrow1) 1.8e+02)) 8e+01 "TraceTypeQuery1" false 0 "None"))
  (if _returnvalue_2
    (for _array_element _outhits
      (Game|Damage|ApplyDamage (.HitActor (Collision|BreakHitResult _array_element)) (Variables|Default|GetSpecialAttackDamage) (Pawn|GetController) 0))))

(event Custom|SetDefense
  ;[1 1 1] 防御
  (if (and (Variables|Default|GetEquip) (not (Variables|Default|GetPlayingDeathMontage)))
    (CallFunction|StopRunning)
    (Variables|Default|SetDefense true)
    (Utilities|FlowControl|Delay (Math|Random|RandomFloatinRange 3.0 5.0))
    (Variables|Default|SetDefense false)))

(event Custom|SetStrafe
  ;[1 1 1] 对峙状态
  (if (and (Variables|Default|GetEquip) (not (Variables|Default|GetPlayingDeathMontage)))
    (Variables|Default|SetStrafe true)
    (AI|Components|Blackboard|SetValueasBool (AI|GetBlackboard self) (Utilities|Name|MakeLiteralName "Strafe") true)))

(event Custom|Run
  ;[1 1 1] 设置跑动和非跑动速度
  (bind _runvalue (Timeline|RunTimeLine Play)
    (:Update
      (Variables|/Script/Engine.CharacterMovementComponent|SetMaxWalkSpeed (Variables|Character|GetCharacterMovement) _runvalue))))

(event Custom|StopRunning
  ;[1 1 1] 设置跑动和非跑动速度
  (bind _runvalue (Timeline|RunTimeLine Reverse)
    (:Update
      (Variables|/Script/Engine.CharacterMovementComponent|SetMaxWalkSpeed (Variables|Character|GetCharacterMovement) _runvalue))))

(event Custom|SpecialAttack
  (bind _returnvalue (Transformation|GetActorForwardVector))
  (bind _target (Variables|Default|GetTarget))
  (bind _target_2 (Variables|Default|GetTarget))
  (bind _target_3 (Variables|Default|GetTarget))
  (bind _returnvalue_2 (Transformation|GetActorLocation _target))
  (bind _returnvalue_3 (Transformation|GetActorLocation _target_3))
  (bind _returnvalue_4 (Transformation|GetActorLocation _target_2))
  ;[1 1 1] 远距离特殊攻击
  (if (and (Variables|Default|GetEquip) (not (Variables|Default|GetPlayingDeathMontage)))
    (Variables|Default|SetAttackMontage true)
    (if (Math|Random|RandomBool)
      (Animation|Montage|PlayMontage (Variables|Character|GetMesh) "/Game/GhostSamurai_Katana/GhostSamurai_Katana/Animation/Apose/Attack/Root/GhostSamurai_APose_JumpAttack02_Root_Montage.GhostSamurai_APose_JumpAttack02_Root_Montage"
        (:then
          (Character|LaunchCharacter (Math|Vector|MakeVector (.x _returnvalue) (.y _returnvalue) 7e+02) true true)
          (Utilities|FlowControl|Delay 0.2)
          (Variables|Default|SetTargetLocation (Math|Vector|MakeVector (+ (.x _returnvalue_4) 2e+02) (.y _returnvalue_4) (+ (.z _returnvalue_4) 2e+01)))
          (Utilities|FlowControl|Sequence
            (:then_0
              (bind _alpha (Timeline|Timeline_1 PlayFromStart)
                (:Update
                  (Transformation|SetActorLocation (Math|Vector|Lerp(Vector) (Transformation|GetActorLocation) (Variables|Default|GetTargetLocation) _alpha) false false))))
            (:then_1
              (Utilities|FlowControl|Delay 0.2)
              (Variables|Default|SetTargetLocation (Math|Vector|MakeVector (+ (.x _returnvalue_2) 2e+02) (.y _returnvalue_2) (+ (.z _returnvalue_2) 2e+01)))))))
      (else
        (Animation|Montage|PlayMontage (Variables|Character|GetMesh) "/Game/GhostSamurai_Katana/GhostSamurai_Katana/Animation/Apose/Attack/Root/GhostSamurai_APose_SPAttack01_Root_Montage.GhostSamurai_APose_SPAttack01_Root_Montage"
          (:then
            (Utilities|FlowControl|Delay 0.9)
            (Variables|Default|SetTargetLocation (Math|Vector|MakeVector (+ (.x _returnvalue_3) 2e+02) (.y _returnvalue_3) (.z (Transformation|GetActorLocation))))
            (bind _alpha_2 (Timeline|Timeline_0 PlayFromStart)
              (:Update
                (Transformation|SetActorLocation (Math|Vector|Lerp(Vector) (Transformation|GetActorLocation) (Variables|Default|GetTargetLocation) _alpha_2) false false)))))))))

(event Custom|ReadyCombat
  ;[1 1 1] 拔剑进入战斗状态
  (Variables|Default|SetEquip true)
  (Variables|Default|SetEquipMontagePlay true)
  (Animation|Montage|PlayMontage (Variables|Character|GetMesh) "/Game/GhostSamurai_Katana/GhostSamurai_Katana/Animation/Common/Root/GhostSamurai_APose_Equip02_Root_Montage.GhostSamurai_APose_Equip02_Root_Montage"
    (:OnBlendOut
      (AI|Components|Blackboard|SetValueasBool (AI|GetBlackboard self) (Utilities|Name|MakeLiteralName "ReadyToFight") true)
      (Variables|Default|SetEquipMontagePlay false)
      (Variables|Default|SetHitMontagePlay false))))

(event Custom|AttackSphere
  (bind _arrow1 (Variables|Default|GetArrow1))
  (bind _returnvalue (Transformation|GetWorldLocation _arrow1))
  ;[1 1 1] 攻击检测
  (bind (_outhits _returnvalue_2) (Collision|MultiSphereTraceByChannel _returnvalue (+ _returnvalue (* (Math|Vector|GetForwardVector _arrow1) 1.5e+02)) 5e+01 "TraceTypeQuery1" false 0 "None"))
  (if _returnvalue_2
    (for _array_element _outhits
      (Game|Damage|ApplyDamage (.HitActor (Collision|BreakHitResult _array_element)) (Variables|Default|GetAttackDamage) (Pawn|GetController) 0))))

(event EventBeginPlay
  (Utilities|FlowControl|Sequence
    (:then_0
      ;[1 1 1] 启动行为树并给黑板赋值
      (AI|RunBehaviorTree (AI|GetAIController self) "/Game/Blueprints/Attack/AI/BT_NegativeAI.BT_NegativeAI")
      (bind _returnvalue (Actor|GetActorOfClass "/Game/Blueprints/BP_BaseCharacter.BP_BaseCharacter_C"))
      (bind _output_get (Variables|Default|SetTarget _returnvalue))
      (AI|Components|Blackboard|SetValueasObject (AI|GetBlackboard self) (Utilities|Name|MakeLiteralName "Target") _output_get))
    (:then_1
      ;[1 1 1] 防御
      (Utilities|Time|SetTimerbyEvent (delegate Custom|SetDefense) (Math|Random|RandomFloatinRange 2e+01 3e+01) true))
    (:then_2
      ;[1 1 1] 对峙状态
      (Utilities|Time|SetTimerbyEvent (delegate Custom|SetStrafe) (Math|Random|RandomFloatinRange 15.0 3e+01) true))
    (:then_3
      ;[1 1 1] 远距离特殊攻击
      (Utilities|Time|SetTimerbyEvent (delegate Custom|SpecialAttack) (Math|Random|RandomFloatinRange 12.0 2e+01) true))
    (:then_4
      ;[1 1 1] 设置HP条
      (bind _aswbp_aihpbar (Utilities|Casting|CastToWBP_AIHPBar (UserInterface|GetUserWidgetObject (Variables|Default|GetHPBar))))
      (Variables|/Game/Blueprints/UI/WBP_AIHPBar.WBP_AIHPBar_C|SetTargetEnemy _aswbp_aihpbar self))))

(event EventTick
  (params (DeltaSeconds :type Float%20%28single-precision%29))
  ;[1 1 1] 启用Tick时修改自身旋转
  (Transformation|SetActorRotation (Math|Interpolation|RInterpTo (Transformation|GetActorRotation) (Math|Rotator|FindLookatRotation (Transformation|GetActorLocation) (Transformation|GetActorLocation (Variables|Default|GetTarget))) (Utilities|Time|GetWorldDeltaSeconds) 25.0))
  (Pawn|Input|AddMovementInput (Transformation|GetActorRightVector) (Variables|Default|GetStrafe%20Value) false))

(event Game|Damage|EventAnyDamage
  (params (Damage :type Float%20%28single-precision%29) (DamageType :type Damage%20Type%20Object%20Reference) (InstigatedBy :type Controller%20Object%20Reference) (DamageCauser :type Actor%20Object%20Reference))
  (bind _hpbar (Variables|Default|GetHPBar))
  ;[1 1 1] 受伤表现
  (Variables|Default|SetAttackMontage false)
  (if (not (Math|Boolean|ORBoolean (Variables|Default|GetDodgeMontagePlay) (Variables|Default|GetPlayingDeathMontage) (Variables|Default|GetEquipMontagePlay)))
    (Variables|Default|SetHitMontagePlay true)
    (if (Variables|Default|GetDefense)
      (Animation|Montage|PlayMontage (Variables|Character|GetMesh) "/Game/GhostSamurai_Katana/GhostSamurai_Katana/Animation/Defense/Root/GhostSamurai_DefenseR_Hit01_Root_Montage.GhostSamurai_DefenseR_Hit01_Root_Montage"
        (:then
          (Utilities|FlowControl|Delay 0.3)
          (Variables|Default|SetHitMontagePlay false)))
      (elif (and (== (Math|Random|RandomIntegerinRange 0 8) 0) (Variables|Default|GetFirstGetHit))
        (Variables|Default|SetDodgeMontagePlay true)
        (Animation|Montage|PlayMontage (Variables|Character|GetMesh) (Utilities|Array|Get(acopy) (Variables|Default|GetDodgeMontages) (Math|Random|RandomIntegerinRange 0 3))
          (:then
            (Utilities|FlowControl|Delay 0.3)
            (Variables|Default|SetHitMontagePlay false))
          (:OnBlendOut
            (Variables|Default|SetDodgeMontagePlay false)
            (Variables|Default|SetHitMontagePlay false)))
        (else
          (Variables|Default|SetFirstGetHit true)
          (if (<= Damage 5e+01)
            _
            (else
              (Animation|Montage|PlayMontage (Variables|Character|GetMesh) "/Game/GhostSamurai_Katana/GhostSamurai_Katana/Animation/Apose/Hit/Root/GhostSamurai_APose_Hit_F_Root_Montage.GhostSamurai_APose_Hit_F_Root_Montage"
                (:then
                  (Utilities|FlowControl|Delay 0.4)
                  (Variables|Default|SetHitMontagePlay false)))))
          (bind _output_get (Variables|Default|SetCurrentHP (Math|Integer|Clamp(Integer) (- (Variables|Default|GetCurrentHP) (Math|Float|Truncate Damage)) 0 (Variables|Default|GetMaxHP))))
          (if (<= _output_get 0)
            (Utilities|IsValid _hpbar
              (:Is%20Valid
                (Components|DestroyComponent _hpbar)
                (Animation|Montage|PlayMontage (Variables|Character|GetMesh) "/Game/GhostSamurai_Katana/GhostSamurai_Katana/Animation/Apose/Die/Root/GhostSamurai_APose_Die01_Root_Montage.GhostSamurai_APose_Die01_Root_Montage"
                  (:then
                    (Variables|Default|SetPlayingDeathMontage true)
                    (Utilities|FlowControl|Delay 0.9)
                    (Physics|SetSimulatePhysics (Variables|Character|GetMesh) true)
                    (Collision|SetCollisionEnabled (Variables|Character|GetMesh) "PhysicsOnly")
                    (Utilities|FlowControl|Delay 3.0)
                    (Actor|DestroyActor)))))))))))

(fn ConstructionScript)