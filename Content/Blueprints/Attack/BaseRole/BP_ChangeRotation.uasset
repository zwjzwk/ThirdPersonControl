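; Anim notify state named "ChangeRotation" that drives character rotation during an animation window.
; On every tick and again at the end, it casts the mesh owner to BP_BaseRole and calls its RInterpToRotation with true.
; The rotation logic itself lives in the role; owners of other classes are ignored.
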(fn GetNotifyName
  (return "ChangeRotation"))

(fn ReceivedNotifyTick
  (params (MeshComp :type Skeletal%20Mesh%20Component%20Object%20Reference) (Animation :type Anim%20Sequence%20Base%20Object%20Reference) (FrameDeltaTime :type Float%20%28single-precision%29))
  (bind _asbp_base_role (Utilities|Casting|CastToBP_BaseRole (Components|GetOwner MeshComp)))
  (Default|RInterptoRotation _asbp_base_role true)
  (return false))

(fn ReceivedNotifyEnd
  (params (MeshComp :type Skeletal%20Mesh%20Component%20Object%20Reference) (Animation :type Anim%20Sequence%20Base%20Object%20Reference))
  (bind _asbp_base_role (Utilities|Casting|CastToBP_BaseRole (Components|GetOwner MeshComp)))
  (Default|RInterptoRotation _asbp_base_role true)
  (return false))