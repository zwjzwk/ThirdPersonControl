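; Base samurai player character for melee combat, with weapon equip, movement, sprint, guard, directional dodge and lock-on.
; Attacks play randomly picked montages gated by state flags, and AttackSphere sphere-traces forward to send damage messages to hit actors.
; Lock-on picks the nearest BP_NegativeAI and interpolates the control rotation toward it on Tick.
; Incoming non-special damage plays a guard or normal hit montage unless dodging.
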(event Custom|ResetAttackMontage
  ;[1 1 1] 攻击
  (Variables|Default|SetAttackMontage false))

(event Custom|AttackSphere
  (bind _arrow1 (Variables|Default|GetArrow1))
  (bind _returnvalue (Transformation|GetWorldLocation _arrow1))
  ;[1 1 1] 攻击检测
  (bind (_outhits _returnvalue_2) (Collision|MultiSphereTraceByChannel _returnvalue (+ _returnvalue (* (Math|Vector|GetForwardVector _arrow1) 1.5e+02)) 5e+01 "TraceTypeQuery1" false 0 "None"))
  (if _returnvalue_2
    (for _array_element _outhits
      (Class|BPIDamage|Damage(Message) (.HitActor (Collision|BreakHitResult _array_element)) 2e+01 false))))

(event EventDamage
  (params (Damage :type Float%20%28single-precision%29) (SpecialAttack :type Boolean))
  (Variables|Default|SetAttackMontage false)
  (if (not (Variables|Default|GetDodgeMontagePlay))
    (Variables|Default|SetHitMontagePlay true)
    (if (not SpecialAttack)
      (if (Variables|Default|GetDefense)
        (Animation|Montage|PlayMontage (Variables|Character|GetMesh) "/Game/GhostSamurai_Katana/GhostSamurai_Katana/Animation/Defense/Root/GhostSamurai_DefenseR_Hit01_Root_Montage.GhostSamurai_DefenseR_Hit01_Root_Montage"
          (:then
            (Utilities|FlowControl|Delay 0.3)))
        (else
          (Animation|Montage|PlayMontage (Variables|Character|GetMesh) "/Game/GhostSamurai_Katana/GhostSamurai_Katana/Animation/Apose/Hit/Root/GhostSamurai_APose_Hit_F_Root_Montage.GhostSamurai_APose_Hit_F_Root_Montage"
            (:then
              (Utilities|FlowControl|Delay 0.3)))))
      (Variables|Default|SetHitMontagePlay false))))

(event EventBeginPlay
  (bind _targetwithdistance (Variables|Default|GetTargetWithDistance))
  ;[1 1 1] BeginPlay
  (Utilities|Map|Clear (Variables|Default|GetTargetWithDistance))
  (bind _outactors (Actor|GetAllActorsOfClass "/Game/Blueprints/Attack/AI/BP_NegativeAI.BP_NegativeAI_C"))
  (for _array_element _outactors
    (Utilities|Map|Add (Variables|Default|GetTargetWithDistance) _array_element (Transformation|GetDistanceTo _array_element self)))
  (bind _keys (Utilities|Map|Keys _targetwithdistance))
  (bind _values (Utilities|Map|Values _targetwithdistance))
  (Variables|Default|SetTarget (Utilities|Array|Get(acopy) _keys (.IndexOfMinValue (Math|Float|MinOfFloatArray _values)))))

(event EventTick
  (params (DeltaSeconds :type Float%20%28single-precision%29))
  (bind _returnvalue (Transformation|GetActorLocation))
  (bind _target (Variables|Default|GetTarget))
  (bind _returnvalue_2 (Transformation|GetActorLocation _target))
  (bind _returnvalue_3 (Math|Rotator|FindLookatRotation _returnvalue _returnvalue_2))
  ;[1 1 1] Tick
  (Utilities|FlowControl|Sequence
    (:then_0
      (CallFunction|CalculateLastInput)
      (if (> (Math|Vector|VectorLength (Transformation|GetVelocity)) 0.0)
        (Variables|/Script/Engine.CharacterMovementComponent|SetbOrientRotationToMovement (Variables|Character|GetCharacterMovement) false)
        (else
          (Variables|/Script/Engine.CharacterMovementComponent|SetbOrientRotationToMovement (Variables|Character|GetCharacterMovement) true))))
    (:then_1
      (if (Variables|Default|GetLock)
        (Utilities|IsValid _target
          (:Is%20Valid
            (Pawn|SetControlRotation (Pawn|GetController) (Math|Interpolation|RInterpTo (Pawn|GetControlRotation :!class /Script/Engine.Pawn) (Math|Rotator|MakeRotator (.roll _returnvalue_3) (+ (.pitch _returnvalue_3) -3e+01) (.yaw _returnvalue_3)) (Utilities|Time|GetWorldDeltaSeconds) 2e+01))))))))

(event Input|ActionEvents|InputActionRun
  (params (Key :type Key%20Structure :default "None"))
  ;[1 1 1] 移动与防御
  (:Pressed
    (if (not (Variables|Default|GetDefense))
      (Variables|Default|SetRun true)
      (bind _runvalue (Timeline|RunTimeLine Play)
        (:Update
          (Variables|/Script/Engine.CharacterMovementComponent|SetMaxWalkSpeed (Variables|Character|GetCharacterMovement) _runvalue)))))
  (:Released
    (Variables|Default|SetRun false)
    (Timeline|RunTimeLine Reverse)))

(event Input|ActionEvents|InputActionDefense
  (params (Key :type Key%20Structure :default "None"))
  ;[1 1 1] 移动与防御
  (:Pressed
    (if (Variables|Default|GetRun)
      (Utilities|FlowControl|Sequence
        (:then_0
          (Variables|Default|SetRun false)
          (bind _runvalue (Timeline|RunTimeLine Reverse)
            (:Update
              (Variables|/Script/Engine.CharacterMovementComponent|SetMaxWalkSpeed (Variables|Character|GetCharacterMovement) _runvalue))))
        (:then_1
          (Variables|Default|SetDefense true :!label _label)))
      (else
        (goto _label))))
  (:Released
    (Variables|Default|SetDefense false)))

(event Input|ActionEvents|InputActionDodge
  (params (Key :type Key%20Structure :default "None"))
  (bind _returnvalue (Input|AxisValues|GetMoveForward))
  (bind _returnvalue_2 (Input|AxisValues|GetMoveRight))
  ;[1 1 1] 翻滚
  (:Pressed
    (if (Variables|Default|GetEquip)
      (if (not (or (Variables|Default|GetDodgeMontagePlay) (Variables|Default|GetAttackMontage)))
        (Variables|Default|SetDodgeMontagePlay true)
        (if (!= _returnvalue 0.0)
          (if (> _returnvalue 0.0)
            (Animation|Montage|PlayMontage (Variables|Character|GetMesh) "/Game/GhostSamurai_Katana/GhostSamurai_Katana/Animation/Apose/Dodge/Root/GhostSamurai_APose_Dodge_F_Root_Montage.GhostSamurai_APose_Dodge_F_Root_Montage" 1.2
              (:OnBlendOut
                _))
            (else
              (Animation|Montage|PlayMontage (Variables|Character|GetMesh) "/Game/GhostSamurai_Katana/GhostSamurai_Katana/Animation/Apose/Dodge/Root/GhostSamurai_APose_Dodge_B_Root_Montage.GhostSamurai_APose_Dodge_B_Root_Montage" 1.2 :!label _label
                (:OnBlendOut
                  _))))
          (elif (!= _returnvalue_2 0.0)
            (if (> _returnvalue_2 0.0)
              (Animation|Montage|PlayMontage (Variables|Character|GetMesh) "/Game/GhostSamurai_Katana/GhostSamurai_Katana/Animation/Apose/Dodge/Root/GhostSamurai_APose_Dodge_R_Root_Montage.GhostSamurai_APose_Dodge_R_Root_Montage" 1.2
                (:OnBlendOut
                  _))
              (else
                (Animation|Montage|PlayMontage (Variables|Character|GetMesh) "/Game/GhostSamurai_Katana/GhostSamurai_Katana/Animation/Apose/Dodge/Root/GhostSamurai_APose_Dodge_L_Root_Montage.GhostSamurai_APose_Dodge_L_Root_Montage" 1.2
                  (:OnBlendOut
                    _))))
            (else
              (goto _label))))
        (Variables|Default|SetDodgeMontagePlay false)))))

(event Input|ActionEvents|InputActionAttack
  (params (Key :type Key%20Structure :default "None"))
  ;[1 1 1] 攻击
  (:Pressed
    (if (Variables|Default|GetEquip)
      (if (and (not (Variables|Default|GetDodgeMontagePlay)) (not (Variables|Default|GetAttackMontage)))
        (Utilities|FlowControl|Sequence
          (:then_0
            (Variables|Default|SetAttackMontage true)
            (bind _output_get (Variables|Default|SetAttackInt (Math|Random|RandomIntegerinRange 0 4)))
            (if (== _output_get (Variables|Default|GetCurrentAttackInt))
              (if (== (Variables|Default|GetAttackInt) 0)
                (bind _result (Math|Integer|IncrementInt (Variables|Default|GetAttackInt))
                  (:%20%20
                    (Variables|Default|SetCurrentAttackInt _result)))
                (else
                  (bind _result_2 (Math|Integer|DecrementInt (Variables|Default|GetAttackInt))
                    (:%20%20
                      (Variables|Default|SetCurrentAttackInt _result_2)))))
              (else
                (Variables|Default|SetCurrentAttackInt _output_get)))
            (Animation|Montage|PlayMontage (Variables|Character|GetMesh) (Utilities|Array|Get(acopy) (Variables|Default|GetAttack%20Montage%20to%20Play) (Variables|Default|GetCurrentAttackInt)))))))))

(event Input|ActionEvents|InputActionLock
  (params (Key :type Key%20Structure :default "None"))
  (bind _targetwithdistance (Variables|Default|GetTargetWithDistance))
  ;[1 1 1] 锁定
  (:Pressed
    (Utilities|FlowControl|FlipFlop
      (:A
        (Variables|Default|SetLock true)
        (Utilities|Map|Clear (Variables|Default|GetTargetWithDistance))
        (bind _outactors (Actor|GetAllActorsOfClass "/Game/Blueprints/Attack/AI/BP_NegativeAI.BP_NegativeAI_C"))
        (for _array_element _outactors
          (Utilities|Map|Add (Variables|Default|GetTargetWithDistance) _array_element (Transformation|GetDistanceTo _array_element self)))
        (bind _keys (Utilities|Map|Keys _targetwithdistance))
        (bind _values (Utilities|Map|Values _targetwithdistance))
        (Variables|Default|SetTarget (Utilities|Array|Get(acopy) _keys (.IndexOfMinValue (Math|Float|MinOfFloatArray _values)))))
      (:B
        (Variables|Default|SetLock false)))))

(event Input|AxisEvents|InputAxisMouseX
  (params (AxisValue :type Float%20%28single-precision%29))
  ;[1 1 1] 移动与防御
  (if (not (Variables|Default|GetLock))
    (Pawn|Input|AddControllerYawInput AxisValue)))

(event Input|AxisEvents|InputAxisMouseY
  (params (AxisValue :type Float%20%28single-precision%29))
  ;[1 1 1] 移动与防御
  (if (not (Variables|Default|GetLock))
    (Pawn|Input|AddControllerPitchInput (* AxisValue -1.0))))

(event Input|AxisEvents|InputAxisMoveRight
  (params (AxisValue :type Float%20%28single-precision%29))
  ;[1 1 1] 移动与防御
  (Pawn|Input|AddMovementInput (Math|Vector|GetRightVector (Math|Rotator|MakeRotator 0.0 0.0 (.yaw (Pawn|GetControlRotation :!class /Script/Engine.Pawn)))) AxisValue false))

(event Input|AxisEvents|InputAxisMoveForward
  (params (AxisValue :type Float%20%28single-precision%29))
  ;[1 1 1] 移动与防御
  (Pawn|Input|AddMovementInput (Math|Vector|GetForwardVector (Math|Rotator|MakeRotator 0.0 0.0 (.yaw (Pawn|GetControlRotation :!class /Script/Engine.Pawn)))) AxisValue false))

(event Input|KeyboardEvents|1
  (params (Key :type Key%20Structure :default "None"))
  ;[1 1 1] 装备武器
  (:Pressed
    (Utilities|FlowControl|DoOnce false
      (:Completed
        (Animation|Montage|PlayMontage (Variables|Character|GetMesh) "/Game/GhostSamurai_Katana/GhostSamurai_Katana/Animation/Common/Root/GhostSamurai_APose_Equip02_Root_Montage.GhostSamurai_APose_Equip02_Root_Montage"
          (:then
            (Utilities|FlowControl|Delay 0.5)
            (Class|BPIReadytoFight|Ready(Message) (Variables|Default|GetTarget)))
          (:OnBlendOut
            (Variables|Default|SetEquip true)))))))

(fn ConstructionScript)

(fn CalculateLastInput
  (bind _charactermovement (Variables|Character|GetCharacterMovement))
  (bind _returnvalue (Pawn|Components|PawnMovement|GetLastInputVector _charactermovement))
  (bind _output_get (Variables|Default|SetInput? (Class|KismetMathLibrary|NotEqualExactlyVectorVector _returnvalue "0, 0, 0")))
  (Variables|Default|SetLastInput _returnvalue)
  (if _output_get
    (Variables|Default|SetLastRotation (Math|Rotator|MakeRotfromX _returnvalue))))

(fn RInterptoRotation
  (params (IsInterp? :type Boolean))
  (if IsInterp?
    (Transformation|SetActorRotation (Math|Interpolation|RInterpTo (Transformation|GetActorRotation) (Variables|Default|GetLastRotation) (Utilities|Time|GetWorldDeltaSeconds) 2e+01))))