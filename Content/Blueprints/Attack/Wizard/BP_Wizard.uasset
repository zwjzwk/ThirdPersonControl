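; Wizard enemy character, driven by an AI controller and blackboard, with an HP bar widget and a magic ball attack.
; Damage lowers clamped HP and briefly sets the BeingAttack blackboard key via a timer, which Tick mirrors into ABP_Wizard's BeingHit.
; At zero HP it removes the bar, plays a death montage, ragdolls, unpossesses and is destroyed.
; MagicAttack spawns BP_MagicBall at a given location, yawed 90 degrees from the mesh.
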(event Custom|MagicAttack
  (params (LeftOrRight :type Vector))
  (bind _mesh (Variables|Character|GetMesh))
  (bind _returnvalue (Transformation|GetWorldRotation _mesh))
  (Game|SpawnActorfromClass "/Game/Blueprints/Attack/Wizard/BP_MagicBall.BP_MagicBall_C" (Math|Transform|MakeTransform LeftOrRight (Math|Rotator|MakeRotator (.roll _returnvalue) (.pitch _returnvalue) (+ (.yaw _returnvalue) 9e+01)) "0.500000,0.500000,0.500000") "Undefined" 0 0))

(event Custom|NotBeingDamaged
  (AI|Components|Blackboard|SetValueasBool (AI|GetBlackboard (AI|GetAIController self)) (Utilities|Name|MakeLiteralName "BeingAttack") false))

(event EventBeginPlay
  (Variables|/Script/Engine.CharacterMovementComponent|SetMaxWalkSpeed (Variables|Character|GetCharacterMovement) 1e+02)
  (bind _aswbp_wizard_hpbar (Utilities|Casting|CastToWBP_WizardHPBar (UserInterface|GetUserWidgetObject (Variables|Default|GetHPBar))))
  (Variables|/Game/Blueprints/UI/WBP_WizardHPBar.WBP_WizardHPBar_C|SetTargetEnemy _aswbp_wizard_hpbar self)
  (bind _asabp_wizard (Utilities|Casting|CastToABP_Wizard (Components|SkeletalMesh|GetAnimInstance (Variables|Character|GetMesh))))
  (Variables|Default|SetABPWizard _asabp_wizard))

(event Game|Damage|EventAnyDamage
  (params (Damage :type Float%20%28single-precision%29) (DamageType :type Damage%20Type%20Object%20Reference) (InstigatedBy :type Controller%20Object%20Reference) (DamageCauser :type Actor%20Object%20Reference))
  (bind _hpbar (Variables|Default|GetHPBar))
  (bind _output_get (Variables|Default|SetCurrentHP (Math|Integer|Clamp(Integer) (- (Variables|Default|GetCurrentHP) (Math|Float|Truncate Damage)) 0 (Variables|Default|GetMaxHP))))
  (if (<= _output_get 0)
    (Actor|Tick|SetActorTickEnabled false)
    (Utilities|IsValid _hpbar
      (:Is%20Valid
        (Components|DestroyComponent _hpbar)
        (Animation|Montage|PlayMontage (Variables|Character|GetMesh) "/Game/Assets/AIAnimations/GhostSamurai_APose_Die01_Root_Montage.GhostSamurai_APose_Die01_Root_Montage"
          (:then
            (Variables|Default|SetPlayingDeathMontage true)
            (Utilities|FlowControl|Delay 0.9)
            (Physics|SetSimulatePhysics (Variables|Character|GetMesh) true)
            (Collision|SetCollisionEnabled (Variables|Character|GetMesh) "PhysicsOnly")
            (Pawn|UnPossess (AI|GetAIController self))
            (Utilities|Time|ClearTimerbyFunctionName 0 "NotBeingDamaged")
            (Utilities|FlowControl|Delay 3.0)
            (Actor|DestroyActor)))))
    (else
      (Utilities|Time|ClearTimerbyFunctionName 0 "NotBeingDamaged")
      (AI|Components|Blackboard|SetValueasBool (AI|GetBlackboard (AI|GetAIController self)) (Utilities|Name|MakeLiteralName "BeingAttack") true)
      (Utilities|Time|SetTimerbyFunctionName 0 "NotBeingDamaged" 0.1 true))))

(event EventTick
  (params (DeltaSeconds :type Float%20%28single-precision%29))
  (Variables|/Game/Blueprints/Attack/Wizard/ABP_Wizard.ABP_Wizard_C|SetBeingHit? (Variables|Default|GetABPWizard) (ScalableFloat|GetValueasBool (AI|GetBlackboard (AI|GetAIController self)) (Utilities|Name|MakeLiteralName "BeingAttack"))))

(fn ConstructionScript)