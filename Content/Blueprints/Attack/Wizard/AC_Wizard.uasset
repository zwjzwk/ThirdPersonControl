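; AC_Wizard is the AI controller for the Wizard, driving it with the BT_Wizard behavior tree.
; On BeginPlay it starts the tree and caches the first player's character as a BP_BaseCharacter.
; When its PawnSensing component sees that player, it writes the player to the AttackTarget blackboard key.
; Nothing in this controller clears the target afterward.
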(event OnSeePawn(PawnSensing)
  (params (Pawn :type Pawn%20Object%20Reference))
  (bind _player (Variables|Default|GetPlayer))
  (if (== Pawn _player)
    (AI|Components|Blackboard|SetValueasObject (Variables|Default|GetBlackboard) (Variables|Default|GetAttackTarget) _player)))

(event EventBeginPlay
  (AI|RunBehaviorTree "/Game/Blueprints/Attack/Wizard/BT_Wizard.BT_Wizard")
  (bind _asbp_base_character (Utilities|Casting|CastToBP_BaseCharacter (Game|GetPlayerCharacter 0)))
  (Variables|Default|SetPlayer _asbp_base_character))

(fn ConstructionScript)