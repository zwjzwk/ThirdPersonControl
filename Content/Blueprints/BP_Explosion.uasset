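; BP_Explosion is a short-lived explosion actor that pushes and damages what is around it when it spawns.
; On BeginPlay it fires its RadialForce impulse and sets a lifespan of a few seconds for self-cleanup.
; A multi sphere trace on the Visibility channel then applies flat damage, without distance falloff, to each hit that casts to BP_BaseCharacter or BP_Enemy.
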(event EventBeginPlay
  (bind _returnvalue (Transformation|GetActorLocation))
  (Class|RadialForceComponent|FireImpulse (Variables|Default|GetRadialForce))
  (Actor|SetLifeSpan 3.0)
  (bind _outhits (Collision|MultiSphereTraceByChannel _returnvalue (+ _returnvalue "0, 0,10.000000") 8e+02 "TraceTypeQuery1" false 0 "None"))
  (for _array_element _outhits
    (bind _asbp_base_character (Utilities|Casting|CastToBP_BaseCharacter (.HitActor (Collision|BreakHitResult _array_element)))
      (:then
        (Game|Damage|ApplyDamage _asbp_base_character 8e+01 0 0))
      (:CastFailed
        (bind _asbp_enemy (Utilities|Casting|CastToBP_Enemy (.HitActor (Collision|BreakHitResult _array_element))))
        (Game|Damage|ApplyDamage _asbp_enemy 8e+01 0 0)))))

(fn ConstructionScript)