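; BP_BaseProjectile is a short-lived projectile, apparently a base class, that destroys itself shortly after spawning.
; When its StaticMesh overlaps any actor other than its owner, it applies point damage using BulletDamage and reversed velocity as hit direction, then destroys itself.
; Blocking hits on physics-simulating components add a velocity-scaled impulse at the projectile's location.
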(event OnComponentBeginOverlap(StaticMesh)
  (params (OverlappedComponent :type Primitive%20Component%20Object%20Reference) (OtherActor :type Actor%20Object%20Reference) (OtherComp :type Primitive%20Component%20Object%20Reference) (OtherBodyIndex :type Integer) (bFromSweep :type Boolean) (SweepResult :type Hit%20Result%20Structure%20%28by%20ref%29))
  (if (!= OtherActor (Components|GetOwner))
    (Game|Damage|ApplyPointDamage OtherActor (Variables|Default|GetBulletDamage) (* (Math|Vector|Normalize (Transformation|GetVelocity)) -1.0) SweepResult)
    (Actor|DestroyActor)))

(event EventBeginPlay
  (Utilities|FlowControl|Delay 0.4)
  (Actor|DestroyActor))

(event Collision|EventActorBeginOverlap
  (params (OtherActor :type Actor%20Object%20Reference)))

(event EventTick
  (params (DeltaSeconds :type Float%20%28single-precision%29)))

(event Collision|EventHit
  (params (MyComp :type Primitive%20Component%20Object%20Reference) (Other :type Actor%20Object%20Reference) (OtherComp :type Primitive%20Component%20Object%20Reference) (bSelfMoved :type Boolean) (HitLocation :type Vector :default "0, 0, 0") (HitNormal :type Vector :default "0, 0, 0") (NormalImpulse :type Vector :default "0, 0, 0") (Hit :type Hit%20Result%20Structure%20%28by%20ref%29))
  (if (Physics|IsSimulatingPhysics OtherComp "None")
    (Physics|AddImpulseatLocation OtherComp (* (Transformation|GetVelocity) 8e+01) (Transformation|GetActorLocation) "None")))

(fn ConstructionScript)