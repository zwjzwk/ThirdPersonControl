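; BP_Grenade is a grenade actor that detonates on a four-second fuse timer or when its static mesh overlaps a base character or enemy.
; The shared Explosion event spawns BP_Explosion at the grenade's transform and plays a loud explosion cue.
; The grenade destroys itself after a short delay, and nothing guards against Explosion firing again during that window.
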(event OnComponentBeginOverlap(StaticMesh)
  (params (OverlappedComponent :type Primitive%20Component%20Object%20Reference) (OtherActor :type Actor%20Object%20Reference) (OtherComp :type Primitive%20Component%20Object%20Reference) (OtherBodyIndex :type Integer) (bFromSweep :type Boolean) (SweepResult :type Hit%20Result%20Structure%20%28by%20ref%29))
  (Utilities|Casting|CastToBP_BaseCharacter OtherActor
    (:then
      _)
    (:CastFailed
      (Utilities|Casting|CastToBP_Enemy OtherActor)))
  (CallFunction|Explosion))

(event Custom|Explosion
  (Game|SpawnActorfromClass "/Game/Blueprints/BP_Explosion.BP_Explosion_C" (Transformation|GetActorTransform) "Undefined" 0 0)
  (Audio|PlaySoundatLocation "/Game/StarterContent/Audio/Explosion_Cue.Explosion_Cue" (Transformation|GetActorLocation) "0, 0, 0" 2.0 1.0 0.0 0 0 0)
  (Utilities|FlowControl|Delay 0.2)
  (Actor|DestroyActor))

(event EventBeginPlay
  (Utilities|Time|SetTimerbyEvent (delegate Custom|Explosion) 4.0))

(fn ConstructionScript
  (|CallParentFunction))