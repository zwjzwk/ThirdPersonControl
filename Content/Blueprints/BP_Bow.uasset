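; Bow weapon, a child of a base weapon Blueprint, that shows its nocked arrow and a quiver of remaining arrows on the character.
; The Arrow bone is hidden when the chamber starts empty or on fire release, and unhidden by the reload montage notify.
; GetWeapon spawns the ClipAmmo quiver on the owner's pelvis socket without physics or collision.
; On pickup and reload, numbered quiver bones above the ammo reserve count are hidden, up to ten.
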(event Custom|SetArrowInQuiver
  (bind _owning_character (Variables|Default|GetOwning%20Character))
  (bind _ammoreserve (Variables|/Game/Blueprints/BP_BaseCharacter.BP_BaseCharacter_C|GetAmmoReserve _owning_character))
  (bind _value (Utilities|Map|Find _ammoreserve "NewEnumerator3"))
  (if (< _value 10)
    (for _index (range (+ _value 1) 10)
      (Components|SkinnedMesh|HideBonebyName (Variables|/Game/Blueprints/BP_ClipAmmo.BP_ClipAmmo_C|GetSkeletalMesh (Variables|Default|GetQuiver)) (Utilities|String|StringToName (Utilities|String|ToString(Integer) _index)) "PBO_None"))))

(event EventBeginPlay
  (|CallParentFunction)
  (if (== (Variables|Default|GetRoundsInChamber) 0)
    (Components|SkinnedMesh|HideBonebyName (Variables|Default|GetSkeletalMesh) "Arrow" "PBO_None")))

(event Collision|EventActorBeginOverlap
  (params (OtherActor :type Actor%20Object%20Reference)))

(event EventTick
  (params (DeltaSeconds :type Float%20%28single-precision%29))
  (|CallParentFunction DeltaSeconds) ; This node is disabled and will not be called.\nDrag off pins to build functionality.
)

(event EventOnWeaponReloadMontageNotify
  (Components|SkinnedMesh|UnHideBonebyName (Variables|Default|GetSkeletalMesh) "Arrow")
  (CallFunction|SetArrowinQuiver))

(event EventGetWeapon
  (params (OwningCharacter :type BP%20Base%20Character%20Object%20Reference))
  (bind _mesh (Variables|/Script/Engine.Character|GetMesh OwningCharacter))
  (|CallParentFunction OwningCharacter)
  (bind _returnvalue (Game|SpawnActorfromClass (Variables|Default|GetClipAmmo) (Transformation|GetSocketTransform _mesh "PelvisSocket" "RTS_World") "AlwaysSpawn" 0 OwningCharacter))
  (bind _output_get (Variables|Default|SetQuiver _returnvalue))
  (Physics|SetSimulatePhysics (Variables|/Game/Blueprints/BP_ClipAmmo.BP_ClipAmmo_C|GetSkeletalMesh _output_get) false)
  (Collision|SetCollisionEnabled (Variables|/Game/Blueprints/BP_ClipAmmo.BP_ClipAmmo_C|GetSkeletalMesh _output_get) "NoCollision")
  (Transformation|AttachComponentToComponent _output_get _mesh "PelvisSocket" "SnapToTarget" "SnapToTarget" "SnapToTarget" true)
  (CallFunction|SetArrowinQuiver))

(event EventFireReleased
  (|CallParentFunction)
  (Components|SkinnedMesh|HideBonebyName (Variables|Default|GetSkeletalMesh) "Arrow" "PBO_None"))

(fn ConstructionScript
  (|CallParentFunction))