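; Base weapon actor for the player's guns and bow, handling firing, fire-mode switching, reloads and magazine/chamber ammo.
; Each fire mode plays RPM-scaled character and weapon montages, whose notifies fire shots and blend-outs chamber rounds or repeat burst and full-auto.
; Shots spawn ammo-specific projectiles per pellet with spread, aimed at the owner's look-at point or along the muzzle at extreme yaw.
; Charge fire scales bow velocity by a "Power" animation curve sampled on release.
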(event Custom|MagReloadWeapon
  (Animation|Montage|PlayMontage (Variables|Default|GetSkeletalMesh) (Variables|Default|GetMagReloadWeap)
    (:OnNotifyBegin
      (CallFunction|OnWeaponReloadMontageNotify))))

(event Custom|Fire
  (bind _rpm (Variables|Default|GetRPM))
  (bind _rpm_2 (Variables|Default|GetRPM))
  (bind _rpm_3 (Variables|Default|GetRPM))
  (bind _rpm_4 (Variables|Default|GetRPM))
  (bind _rpm_5 (Variables|Default|GetRPM))
  (bind _rpm_6 (Variables|Default|GetRPM))
  (bind _returnvalue (/ _rpm 45.0))
  (bind _returnvalue_2 (/ _rpm_3 45.0))
  (bind _returnvalue_3 (/ _rpm_2 2e+02))
  (bind _returnvalue_4 (/ _rpm_5 45.0))
  (bind _returnvalue_5 (/ _rpm_4 2e+02))
  (bind _returnvalue_6 (/ _rpm_6 2e+02))
  (Variables|Default|SetFiring true)
  (switch Utilities|FlowControl|Switch|SwitchonEFireMode (Variables|Default|GetFireMode)
    (:NewEnumerator0
      (Animation|Montage|PlayMontage (Variables|/Script/Engine.Character|GetMesh (Variables|Default|GetOwning%20Character)) "/Game/Assets/Character/Animations/A_2HW_ADS_Fire_Montage.A_2HW_ADS_Fire_Montage" _returnvalue_4
        (:then
          (Animation|Montage|PlayMontage (Variables|Default|GetSkeletalMesh) (Variables|Default|GetFireMontageWeapon) _returnvalue_4
            (:OnBlendOut
              (Animation|Montage|PlayMontage (Variables|/Script/Engine.Character|GetMesh (Variables|Default|GetOwning%20Character)) (Variables|Default|GetManualChargeMontageChar) _returnvalue
                (:then
                  (Animation|Montage|PlayMontage (Variables|Default|GetSkeletalMesh) (Variables|Default|GetManualChargeMontageWeap) _returnvalue
                    (:OnBlendOut
                      (CallFunction|Chambering))))))
            (:OnNotifyBegin
              (CallFunction|WeaponFire))))))
    (:NewEnumerator1
      (Utilities|FlowControl|DoOnce false :!label _label
        (:Completed
          (Animation|Montage|PlayMontage (Variables|/Script/Engine.Character|GetMesh (Variables|Default|GetOwning%20Character)) "/Game/Assets/Character/Animations/A_2HW_ADS_Fire_Montage.A_2HW_ADS_Fire_Montage" _returnvalue_5
            (:then
              (Animation|Montage|PlayMontage (Variables|Default|GetSkeletalMesh) (Variables|Default|GetFireMontageWeapon) _returnvalue_5
                (:OnBlendOut
                  (CallFunction|Chambering)
                  (goto _label Reset))
                (:OnNotifyBegin
                  (CallFunction|WeaponFire))))))))
    (:NewEnumerator2
      (Animation|Montage|PlayMontage (Variables|/Script/Engine.Character|GetMesh (Variables|Default|GetOwning%20Character)) "/Game/Assets/Character/Animations/A_2HW_ADS_Fire_Montage.A_2HW_ADS_Fire_Montage" _returnvalue_3
        (:then
          (Animation|Montage|PlayMontage (Variables|Default|GetSkeletalMesh) (Variables|Default|GetFireMontageWeapon) _returnvalue_3
            (:OnBlendOut
              (CallFunction|Chambering)
              (CallFunction|ShouldRepeatCheck))
            (:OnNotifyBegin
              (CallFunction|WeaponFire)
              (Math|Integer|IncrementInt (Variables|Default|GetBursts)))))))
    (:NewEnumerator3
      (Animation|Montage|PlayMontage (Variables|/Script/Engine.Character|GetMesh (Variables|Default|GetOwning%20Character)) "/Game/Assets/Character/Animations/A_2HW_ADS_Fire_Montage.A_2HW_ADS_Fire_Montage" _returnvalue_6
        (:then
          (Animation|Montage|PlayMontage (Variables|Default|GetSkeletalMesh) (Variables|Default|GetFireMontageWeapon) _returnvalue_6
            (:OnBlendOut
              (CallFunction|Chambering)
              (CallFunction|ShouldRepeatCheck))
            (:OnNotifyBegin
              (CallFunction|WeaponFire))))))
    (:NewEnumerator4
      (Animation|Montage|PlayMontage (Variables|/Script/Engine.Character|GetMesh (Variables|Default|GetOwning%20Character)) "/Game/Assets/Character/Animations/A_Bow_Draw_ChargeOnly_Char_Montage.A_Bow_Draw_ChargeOnly_Char_Montage" _returnvalue_2
        (:then
          (Animation|Montage|PlayMontage (Variables|Default|GetSkeletalMesh) "/Game/Assets/Weapons/Bow/A_Bow_Draw_ChargeOnly_Montage.A_Bow_Draw_ChargeOnly_Montage" _returnvalue_2
            (:then
              (Variables|/Game/Blueprints/BP_BaseCharacter.BP_BaseCharacter_C|SetCharging (Variables|Default|GetOwning%20Character) true))))))))

(event Custom|BCRReloadStopWeapon
  (Animation|Montage|PlayMontage (Variables|Default|GetSkeletalMesh) (Variables|Default|GetBCRReloadWeap) 1.0 0.0 "End"))

(event Custom|OnWeaponReloadMontageNotify)

(event Custom|StopCharging
  (bind _owning_character (Variables|Default|GetOwning%20Character))
  (Variables|/Game/Blueprints/BP_BaseCharacter.BP_BaseCharacter_C|SetCharging _owning_character false)
  (Animation|Montage|MontageStop (Components|SkeletalMesh|GetAnimInstance (Variables|/Script/Engine.Character|GetMesh _owning_character)) 0.0 "/Game/Assets/Character/Animations/A_Bow_Draw_ChargeOnly_Char_Montage.A_Bow_Draw_ChargeOnly_Char_Montage")
  (Animation|Montage|MontageStop (Components|SkeletalMesh|GetAnimInstance (Variables|Default|GetSkeletalMesh)) 0.0 "/Game/Assets/Weapons/Bow/A_Bow_Draw_ChargeOnly_Montage.A_Bow_Draw_ChargeOnly_Montage"))

(event Custom|FireReleased
  (bind _rpm (Variables|Default|GetRPM))
  (bind _owning_character (Variables|Default|GetOwning%20Character))
  (bind _returnvalue (/ _rpm 45.0))
  (bind _mesh (Variables|/Script/Engine.Character|GetMesh _owning_character))
  (bind _returnvalue_2 (Components|SkeletalMesh|GetAnimInstance _mesh))
  (bind _returnvalue_3 (Animation|Curves|GetCurveValue _returnvalue_2 "Power"))
  (Variables|Default|SetFiring false)
  (Variables|Default|SetBursts 0)
  (switch Utilities|FlowControl|Switch|SwitchonEFireMode (Variables|Default|GetFireMode)
    (:NewEnumerator4
      (if (> _returnvalue_3 0.2)
        (Variables|Default|SetPower _returnvalue_3)
        (Animation|Montage|PlayMontage (Variables|/Script/Engine.Character|GetMesh (Variables|Default|GetOwning%20Character)) "/Game/Assets/Character/Animations/A_Bow_Fire_Char_Montage.A_Bow_Fire_Char_Montage" _returnvalue
          (:then
            (Animation|Montage|PlayMontage (Variables|Default|GetSkeletalMesh) (Variables|Default|GetFireMontageWeapon) _returnvalue
              (:OnNotifyBegin
                (CallFunction|WeaponFire))))
          (:OnBlendOut
            (Variables|/Game/Blueprints/BP_BaseCharacter.BP_BaseCharacter_C|SetCharging (Variables|Default|GetOwning%20Character) false)))
        (else
          (CallFunction|StopCharging))))))

(event Custom|RepeatFire
  (bind _rpm (Variables|Default|GetRPM))
  (bind _rpm_2 (Variables|Default|GetRPM))
  (bind _rpm_3 (Variables|Default|GetRPM))
  (bind _rpm_4 (Variables|Default|GetRPM))
  (bind _rpm_5 (Variables|Default|GetRPM))
  (bind _rpm_6 (Variables|Default|GetRPM))
  (bind _returnvalue (/ _rpm 45.0))
  (bind _returnvalue_2 (/ _rpm_3 45.0))
  (bind _returnvalue_3 (/ _rpm_2 2e+02))
  (bind _returnvalue_4 (/ _rpm_5 45.0))
  (bind _returnvalue_5 (/ _rpm_4 2e+02))
  (bind _returnvalue_6 (/ _rpm_6 2e+02))
  (switch Utilities|FlowControl|Switch|SwitchonEFireMode (Variables|Default|GetFireMode)
    (:NewEnumerator0
      (Animation|Montage|PlayMontage (Variables|/Script/Engine.Character|GetMesh (Variables|Default|GetOwning%20Character)) "/Game/Assets/Character/Animations/A_2HW_ADS_Fire_Montage.A_2HW_ADS_Fire_Montage" _returnvalue_4
        (:then
          (Animation|Montage|PlayMontage (Variables|Default|GetSkeletalMesh) (Variables|Default|GetFireMontageWeapon) _returnvalue_4
            (:OnBlendOut
              (Animation|Montage|PlayMontage (Variables|/Script/Engine.Character|GetMesh (Variables|Default|GetOwning%20Character)) (Variables|Default|GetManualChargeMontageChar) _returnvalue
                (:then
                  (Animation|Montage|PlayMontage (Variables|Default|GetSkeletalMesh) (Variables|Default|GetManualChargeMontageWeap) _returnvalue
                    (:OnBlendOut
                      (CallFunction|Chambering))))))
            (:OnNotifyBegin
              (CallFunction|WeaponFire))))))
    (:NewEnumerator1
      (Utilities|FlowControl|DoOnce false :!label _label
        (:Completed
          (Animation|Montage|PlayMontage (Variables|/Script/Engine.Character|GetMesh (Variables|Default|GetOwning%20Character)) "/Game/Assets/Character/Animations/A_2HW_ADS_Fire_Montage.A_2HW_ADS_Fire_Montage" _returnvalue_5
            (:then
              (Animation|Montage|PlayMontage (Variables|Default|GetSkeletalMesh) (Variables|Default|GetFireMontageWeapon) _returnvalue_5
                (:OnBlendOut
                  (CallFunction|Chambering)
                  (goto _label Reset))
                (:OnNotifyBegin
                  (CallFunction|WeaponFire))))))))
    (:NewEnumerator2
      (Animation|Montage|PlayMontage (Variables|/Script/Engine.Character|GetMesh (Variables|Default|GetOwning%20Character)) "/Game/Assets/Character/Animations/A_2HW_ADS_Fire_Montage.A_2HW_ADS_Fire_Montage" _returnvalue_3
        (:then
          (Animation|Montage|PlayMontage (Variables|Default|GetSkeletalMesh) (Variables|Default|GetFireMontageWeapon) _returnvalue_3
            (:OnBlendOut
              (CallFunction|Chambering)
              (CallFunction|ShouldRepeatCheck))
            (:OnNotifyBegin
              (CallFunction|WeaponFire)
              (Math|Integer|IncrementInt (Variables|Default|GetBursts)))))))
    (:NewEnumerator3
      (Animation|Montage|PlayMontage (Variables|/Script/Engine.Character|GetMesh (Variables|Default|GetOwning%20Character)) "/Game/Assets/Character/Animations/A_2HW_ADS_Fire_Montage.A_2HW_ADS_Fire_Montage" _returnvalue_6
        (:then
          (Animation|Montage|PlayMontage (Variables|Default|GetSkeletalMesh) (Variables|Default|GetFireMontageWeapon) _returnvalue_6
            (:OnBlendOut
              (CallFunction|Chambering)
              (CallFunction|ShouldRepeatCheck))
            (:OnNotifyBegin
              (CallFunction|WeaponFire))))))
    (:NewEnumerator4
      (Animation|Montage|PlayMontage (Variables|/Script/Engine.Character|GetMesh (Variables|Default|GetOwning%20Character)) "/Game/Assets/Character/Animations/A_Bow_Draw_ChargeOnly_Char_Montage.A_Bow_Draw_ChargeOnly_Char_Montage" _returnvalue_2
        (:then
          (Animation|Montage|PlayMontage (Variables|Default|GetSkeletalMesh) "/Game/Assets/Weapons/Bow/A_Bow_Draw_ChargeOnly_Montage.A_Bow_Draw_ChargeOnly_Montage" _returnvalue_2
            (:then
              (Variables|/Game/Blueprints/BP_BaseCharacter.BP_BaseCharacter_C|SetCharging (Variables|Default|GetOwning%20Character) true))))))))

(event Custom|WeaponToggleFireMode
  (if (> (Utilities|Array|Length (Variables|Default|GetAvailableFireMode)) 1)
    (bind _nextitem (Utilities|GetArrayNextItem (Variables|Default|GetAvailableFireMode) (Variables|Default|GetFireMode))
      (:Out
        (bind _output_get (Variables|Default|SetFireMode _nextitem))
        (Development|PrintString (Utilities|String|EnumtoString _output_get))))
    (else
      (Development|PrintString "No Other Fire Mode Available"))))

(event Custom|WeaponFire
  (bind _owning_character (Variables|Default|GetOwning%20Character))
  (bind _skeletalmesh (Variables|Default|GetSkeletalMesh))
  (bind _owning_character_2 (Variables|Default|GetOwning%20Character))
  (bind _skeletalmesh_2 (Variables|Default|GetSkeletalMesh))
  (bind _ammotype (Variables|Default|GetAmmoType))
  (bind _roundsinchamber (Variables|Default|GetRoundsInChamber))
  (bind _skeletalmesh_3 (Variables|Default|GetSkeletalMesh))
  (bind _returnvalue (Transformation|GetSocketRotation _skeletalmesh "Muzzle"))
  (bind _returnvalue_2 (Transformation|GetSocketLocation _skeletalmesh_2 "Muzzle"))
  (bind _returnvalue_3 (Transformation|GetSocketTransform _skeletalmesh_3 "Muzzle" "RTS_World"))
  (bind _returnvalue_4 (Utilities|Select :Index _ammotype :NewEnumerator0 "/Game/Blueprints/BP_BaseProjectile.BP_BaseProjectile_C" :NewEnumerator1 "/Game/Blueprints/BP_BaseProjectile.BP_BaseProjectile_C" :NewEnumerator2 "/Game/Blueprints/BP_BaseProjectile.BP_BaseProjectile_C" :NewEnumerator3 "/Game/Blueprints/BP_Arrow.BP_Arrow_C" :NewEnumerator4 "/Game/Blueprints/BP_Grenade.BP_Grenade_C"))
  (bind _lookatpoint (Variables|/Game/Blueprints/BP_BaseCharacter.BP_BaseCharacter_C|GetLookAtPoint _owning_character))
  (bind _yaw (Variables|/Game/Blueprints/BP_BaseCharacter.BP_BaseCharacter_C|GetYaw _owning_character_2))
  (bind _returnvalue_5 (Math|Vector|GetForwardVector _returnvalue))
  (bind _returnvalue_6 (Math|Float|Absolute(Float) _yaw))
  (bind _returnvalue_7 (- _lookatpoint _returnvalue_2))
  (bind _returnvalue_8 (>= _returnvalue_6 9e+01))
  (bind _returnvalue_9 (Math|Vector|Normalize _returnvalue_7))
  (bind _returnvalue_10 (or _returnvalue_8 false))
  (bind _returnvalue_11 (Math|Vector|SelectVector _returnvalue_5 _returnvalue_9 _returnvalue_10))
  (bind _returnvalue_12 (Math|Conversions|RotationFromXVector _returnvalue_11))
  (|SetBy-RefVar _roundsinchamber (- _roundsinchamber 1))
  (Math|Integer|IncrementInt (Variables|Default|GetShotsFired)
    (:%20%20
      (for _index (range 1 (Variables|Default|GetPelletPerShot))
        (bind _bulletspread (CallFunction|FLBulletSpread (Variables|Default|GetMaxSpreadAngle) (Variables|Default|GetMaxProjectileDistance)))
        (bind _returnvalue_13 (Game|SpawnActorfromClass _returnvalue_4 (Math|Transform|MakeTransform (.location _returnvalue_3) (.rotation _returnvalue_3) (Math|Vector|SelectVector "0.100000,0.100000,0.100000" (.scale _returnvalue_3) (== _returnvalue_4 "/Game/Blueprints/BP_Grenade.BP_Grenade_C"))) "AlwaysSpawn" self 0))
        (bind _asbp_base_projectile (Utilities|Casting|CastToBP_BaseProjectile _returnvalue_13))
        (Utilities|IsValid (Variables|/Game/Blueprints/BP_BaseProjectile.BP_BaseProjectile_C|GetProjectileMovement _asbp_base_projectile)
          (:Is%20Valid
            (Variables|/Script/Engine.MovementComponent|SetVelocity (Variables|/Game/Blueprints/BP_BaseProjectile.BP_BaseProjectile_C|GetProjectileMovement _asbp_base_projectile) (* (Math|Vector|Normalize (+ (* (Math|Vector|GetForwardVector _returnvalue_12) (Variables|Default|GetMaxProjectileDistance)) (* (Math|Vector|GetRightVector _returnvalue_12) (.x _bulletspread)) (* (Math|Vector|GetUpVector _returnvalue_12) (.y _bulletspread)))) (* (Variables|Default|GetMuzzleVelocity) (Utilities|Select :Index (Variables|Default|GetWeaponType) :NewEnumerator0 1.0 :NewEnumerator1 1.0 :NewEnumerator2 1.0 :NewEnumerator4 (Variables|Default|GetPower)))))))))))

(event Custom|MagReloadDone
  (params (RoundsLoaded :type Integer))
  (Variables|Default|SetRoundsInMag RoundsLoaded))

(event Custom|PlayManualChargeAnimation
  (Animation|Montage|PlayMontage (Variables|Default|GetSkeletalMesh) (Variables|Default|GetManualChargeMontageWeap)
    (:OnBlendOut
      (CallFunction|Chambering))))

(event Custom|BCRReloadWeapon
  (Animation|Montage|PlayMontage (Variables|Default|GetSkeletalMesh) (Variables|Default|GetBCRReloadWeap)))

(event Custom|BCRReloadDone
  (params (RoundsLoaded :type Integer))
  (if (== (Variables|Default|GetMagSize) 0)
    (Variables|Default|SetRoundsInChamber (+ (Variables|Default|GetRoundsInChamber) RoundsLoaded))
    (else
      (Variables|Default|SetRoundsInMag (+ RoundsLoaded (Variables|Default|GetRoundsInMag))))))

(event EventFirePressed
  (Variables|Default|SetTesting true)
  (if (> (Variables|Default|GetRoundsInChamber) 0)
    (CallFunction|Fire)))

(event EventGetWeapon
  (params (OwningCharacter :type BP%20Base%20Character%20Object%20Reference))
  (Variables|Default|SetOwning%20Character OwningCharacter)
  (Physics|SetSimulatePhysics (Variables|Default|GetSkeletalMesh) false)
  (Collision|SetCollisionEnabled (Variables|Default|GetSkeletalMesh) "NoCollision")
  (Variables|Default|SetAimBaselineOffset (- (Class|KismetAnimationLibrary|DistanceBetweenTwoSocketsandMapRange (Variables|Default|GetSkeletalMesh) "Root" "RTS_World" "Sight" "RTS_World" false 0.0 0.0 0.0 0.0) 13.512316)))

(event EventTick
  (params (DeltaSeconds :type Float%20%28single-precision%29)))

(fn ConstructionScript)

(fn ShouldRepeatCheck
  (if (Utilities|Select :Index (Variables|Default|GetFireMode) :NewEnumerator0 false :NewEnumerator1 false :NewEnumerator2 (Math|Boolean|ANDBoolean (Variables|Default|GetFiring) (> (Variables|Default|GetRoundsInChamber) 0) (< (Variables|Default|GetBursts) (Variables|Default|GetBurstCount))) :NewEnumerator3 (and (Variables|Default|GetFiring) (> (Variables|Default|GetRoundsInChamber) 0)) :NewEnumerator4 false)
    (CallFunction|RepeatFire)))

(fn Chambering
  (bind _roundsinmag (Variables|Default|GetRoundsInMag))
  (bind _roundsinchamber (Variables|Default|GetRoundsInChamber))
  (if (> (Variables|Default|GetRoundsInMag) 0)
    (|SetBy-RefVar _roundsinmag (- _roundsinmag 1))
    (|SetBy-RefVar _roundsinchamber (+ _roundsinchamber 1))))

(fn GetWeaponPanelInfo
  (return self (Variables|Default|GetWeaponType)))